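; Player vehicle pawn for the Itachigu machine, handling driving input, gun animation and a question-based level and score system.
; Tick checks for every third question, then moves Level down, keeps it or raises it by points earned, within 1–10.
; Each point adds two to the power of Level to the score.
; Helper functions open menu widgets; the looping fire timer calls an empty Shoot, its bullet spawn disconnected.
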(event `self.ReceiveBeginPlay`)

(event `Key|Escape`
  (params (Key :type "Key Structure"))
  (:`Pressed`
    (`KismetSystemLibrary.QuitGame` null "Quit")))

(event `Key|Z`
  (params (Key :type "Key Structure"))
  (:`Pressed`
    (bind _returnvalue (`|CreateWidget` "/Game/UI/exit.exit_C"))
    (`UserWidget.AddToViewport` _returnvalue 0)))

(event `Key|LeftMouseButton`
  (params (Key :type "Key Structure"))
  ;[1 1 1] Gun fire
  (:`Pressed`
    (`|ExecutionSequence`
      (:`then_0`
        (bind _returnvalue (`KismetSystemLibrary.K2_SetTimer` null "Shoot" 0.12 true)))
      (:`then_1`
        (bind _asabp_itachigu_machine (cast `/Game/ItachiguMachine/Blueprints/ABP_ItachiguMachine` (`SkeletalMeshComponent.GetAnimInstance` (`self.Mesh`))))
        (`/Game/ItachiguMachine/Blueprints/ABP_ItachiguMachine.GunFire` _asabp_itachigu_machine))))
  (:`Released`
    (`KismetSystemLibrary.K2_ClearAndInvalidateTimerHandle` _returnvalue)
    (`/Game/ItachiguMachine/Blueprints/ABP_ItachiguMachine.GunStop` _asabp_itachigu_machine)))

(event `InputAxis|MoveRight` :overrideparent false
  (params (AxisValue :type "Float (single-precision)"))
  ;[1 1 1] Steering input
  (bind _output_get (set `self.SteeringValue` AxisValue))
  (`WheeledVehicleMovementComponent.SetSteeringInput` (`self.VehicleMovement`) _output_get))

(event `InputAction|Handbrake`
  (params (Key :type "Key Structure"))
  (bind _vehiclemovement (`self.VehicleMovement`))
  ;[1 1 1] Handbrake input
  (:`Pressed`
    (`WheeledVehicleMovementComponent.SetHandbrakeInput` _vehiclemovement true)
    (bind _asplayer_controller (cast `PlayerController` (`self.GetController`))))
  (:`Released`
    (`WheeledVehicleMovementComponent.SetHandbrakeInput` _vehiclemovement false)))

(event `InputAxis|MoveForward` :overrideparent false
  (params (AxisValue :type "Float (single-precision)"))
  ;[1 1 1] Throttle input
  (`WheeledVehicleMovementComponent.SetThrottleInput` (`self.VehicleMovement`) AxisValue))

(event `SpawnNumber`)

(event `AddPointInLevel`
  (set `self.PointInLevel` (+ (`self.PointInLevel`) 1))
  (`self.ScoreOfPlayer`))

(event `self.ReceiveTick`
  (params (DeltaSeconds :type "Float (single-precision)"))
  (`|ExecutionSequence`
    (:`then_0`
      (if (`self.SpawnNum`)
        (`self.Respawn`)))
    (:`then_1`
      (if (>= (`self.CountQuestion`) 3)
        (`self.LevelCharacter`)
        (set `self.CountQuestion` 0)))))

(event `LevelCharacter`
  (if (== (`self.PointInLevel`) 0)
    (if (== (`self.Level`) 1)
      (set `self.Level` 1)
      (set `self.PointInLevel` 0)
      (elif (> (`self.Level`) 1)
        (set `self.Level` (- (`self.Level`) 1))
        (set `self.PointInLevel` 0)))
    (elif (== (`self.PointInLevel`) 1)
      (set `self.Level` (`self.Level`))
      (set `self.PointInLevel` 0)
      (elif (>= (`self.PointInLevel`) 2)
        (if (>= (`self.Level`) 10)
          (set `self.Level` 10)
          (set `self.PointInLevel` 0)
          (else
            (set `self.Level` (+ (`self.Level`) 1))
            (set `self.PointInLevel` 0)))))))

(event `ScoreOfPlayer`
  (set `self.PlayerScore` (+ (`self.PlayerScore`) (`KismetMathLibrary.FTrunc` (`KismetMathLibrary.MultiplyMultiply_FloatFloat` 2.0 (`KismetMathLibrary.Conv_IntToDouble` (`self.Level`)))))))

(event `ChangeColor`
  (params (Condition :type Boolean))
  (bind _jockey (`self.Jockey`))
  (if Condition
    (`PrimitiveComponent.SetMaterial` _jockey 3 "/Game/ItachiguMachine/Blueprints/NewMaterial.NewMaterial")
    (else
      (`PrimitiveComponent.SetMaterial` _jockey 3 "/Game/ItachiguMachine/Jockey_Character/Materials/MI_GumakoBody.MI_GumakoBody"))))

(event `Key|E`
  (params (Key :type "Key Structure")))

(event `ChangeColorMultiplayer`)

(event `ChangeColorServer`)

(fn `dead`
  (`GameplayStatics.SpawnEmitterAtLocation` null (`self.K2_GetActorLocation`))
  (set `PlayerController.bShowMouseCursor` true (`GameplayStatics.GetPlayerController` 0))
  (bind _returnvalue (`|CreateWidget` "/Game/UI/exit.exit_C" (`GameplayStatics.GetPlayerController` 0)))
  (`UserWidget.AddToViewport` _returnvalue 0))

(fn `deadnumber`
  (`GameplayStatics.SpawnEmitterAtLocation` null (`self.K2_GetActorLocation`))
  (set `PlayerController.bShowMouseCursor` true (`GameplayStatics.GetPlayerController` 0))
  (bind _returnvalue (`|CreateWidget` "/Game/UI/deaddd.deaddd_C" (`GameplayStatics.GetPlayerController` 0)))
  (`UserWidget.AddToViewport` _returnvalue 0))

(fn `newlevel`
  (bind _returnvalue (`|CreateWidget` "/Game/UI/numbermap.numbermap_C" (`GameplayStatics.GetPlayerController` 0)))
  (`UserWidget.AddToViewport` _returnvalue 0))

(fn `Number`
  (`GameplayStatics.OpenLevel` "Maptest1")
  (`GameplayStatics.SetGamePaused` true)
  (bind _returnvalue (`|CreateWidget` "/Game/UI/finisgame.finisgame_C"))
  (`UserWidget.AddToViewport` _returnvalue 0))

(fn `RespawnNumber`
  (returns (`Respawn?` :type Boolean))
  (return true))

(fn `Shoot`)

(fn `start`
  (`GameplayStatics.SpawnEmitterAtLocation` null (`self.K2_GetActorLocation`))
  (set `PlayerController.bShowMouseCursor` true (`GameplayStatics.GetPlayerController` 0))
  (bind _returnvalue (`|CreateWidget` "/Game/UI/startview.startview_C" (`GameplayStatics.GetPlayerController` 0)))
  (`UserWidget.AddToViewport` _returnvalue 0))

(fn `UserConstructionScript`)